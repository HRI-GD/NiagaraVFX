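; BP_TextureBaker is an editor utility actor that bakes a material into a static texture asset.
; Its BakeTexture function checks that the render target and material are valid, then draws the material to the render target.
; It saves the result as a Texture2D through the editor-only render-target conversion, using a fixed asset name.
; The event graph and construction script are empty, so all work happens in that function.
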(fn `BakeTexture`
  (if (and (`KismetSystemLibrary.IsValid` (`self.Texture Render Target`)) (`KismetSystemLibrary.IsValid` (`self.Material`)))
    (`KismetRenderingLibrary.DrawMaterialToRenderTarget` (`self.Texture Render Target`) (`self.Material`))
    (`KismetRenderingLibrary.RenderTargetCreateStaticTexture2DEditorOnly` (`self.Texture Render Target`) "TextureFromRenderTarget")))

(fn `UserConstructionScript`)